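; BP_IANPC is an NPC Blueprint that shows dialogue lines through its Talk event.
; Each Talk call increments DialogueIndex, then prints that entry of the Dialogue array with PrintString if the index is at most the array length.
; The bound check is inclusive, so an index equal to the length reads past the last entry.
; Nothing here resets the index, and the construction script is empty.
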(event `/Game/Blueprints/GameEngien/UI_Talk.Talk`
  (`/Engine/EditorBlueprintResources/StandardMacros.IncrementInt` (`self.dialogueIndex`)
    (:`  `
      (if (<= (`self.dialogueIndex`) (`KismetArrayLibrary.Array_Length` (`self.dialogue`)))
        (`KismetSystemLibrary.PrintString` (`|GetArrayItem` (`self.dialogue`) (`self.dialogueIndex`)))))))

(fn `UserConstructionScript`)