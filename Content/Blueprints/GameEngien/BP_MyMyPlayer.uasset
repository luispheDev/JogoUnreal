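; Player Blueprint that lets the player interact with nearby objects and talk to NPCs by pressing E.
; One E handler scans overlapping actors and sends InteractMessage, with itself as argument, to the first that implements InteractInterface.
; A second E handler calls TalkMessage on every overlapping BP_IANPC, with its UI_Talk interface check left unused.
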(event `Key|E`
  (params (Key :type "Key Structure"))
  (:`Pressed`
    (for _array_element (`self.GetOverlappingActors` "/Script/Engine.Actor")
      (if (`KismetSystemLibrary.DoesImplementInterface` _array_element "/Game/Blueprints/GameEngien/InteractInterface.InteractInterface_C")
        (message `/Game/Blueprints/GameEngien/InteractInterface.Interact` _array_element self)
        (break)))))

(event `Key|E`
  (params (Key :type "Key Structure"))
  (:`Pressed`
    (for _array_element (`self.GetOverlappingActors` "/Game/IA/BP_IANPC.BP_IANPC_C")
      (if true
        (message `/Game/Blueprints/GameEngien/UI_Talk.Talk` _array_element)))))

(fn `UserConstructionScript`)